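; Cannon actor that automatically fires projectiles on a repeating loop from the moment play begins.
; Each cycle waits for the fire-rate delay, then spawns a BP_Projectile at the Arrow component's location and rotation with a configurable scale.
; The Cannon_Fire timeline then animates the barrel along its local Y axis, and its fire-done event restarts the cycle.
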(event EventBeginPlay
  (bind _arrow (Variables|Default|GetArrow))
  (Utilities|FlowControl|Delay (Variables|ProjectileAttributes|GetProjectile%20Firerate) :!label _label)
  (Game|SpawnActorfromClass "/Game/Blueprints/BP_Projectile.BP_Projectile_C" (Math|Transform|MakeTransform (Transformation|GetWorldLocation _arrow) (Transformation|GetWorldRotation _arrow) (Math|Conversions|ToVector(Float) (Variables|ProjectileAttributes|GetProjectile%20Scale))) "Undefined" 0 0)
  (bind _barrelshoottimeline (Timeline|Cannon_Fire PlayFromStart)
    (:Update
      (Transformation|SetRelativeLocation (Variables|Default|GetCanon) (Math|Vector|MakeVector 0.0 _barrelshoottimeline 0.0) false false))
    (:CannonFiredone
      (goto _label))))

(event Collision|EventActorBeginOverlap
  (params (OtherActor :type Actor%20Object%20Reference)))

(event EventTick
  (params (DeltaSeconds :type Float%20%28single-precision%29)))

(fn ConstructionScript)