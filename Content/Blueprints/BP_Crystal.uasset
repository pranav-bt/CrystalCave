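; BP_Crystal is a pickup crystal that flies into the player when touched, shrinking and fading out before it is destroyed.
; On overlap with player pawn 0 it caches its location, scale and light intensity, then plays the LerpAlphaBlend timeline.
; Separate timeline tracks drive lerps toward the pawn's live position, to zero scale and to zero light intensity, and the actor destroys itself on finish.
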(event Collision|EventActorBeginOverlap
  (params (OtherActor :type Actor%20Object%20Reference))
  (Utilities|IsPlayer OtherActor
    (:Player
      (CallFunction|GetStartValues)
      (bind (_direction _location_track _scale_track _light_track) (Timeline|Lerp%20Alpha%20Blend Play)
        (:Update
          (CallFunction|MovetoPawn (Game|Player|GetPlayerPawn 0) _location_track)
          (CallFunction|ScaleCrystal _scale_track)
          (Rendering|Components|Light|SetIntensity (Variables|Default|GetPointLight) (Math|Float|Lerp (Variables|Default|GetStartIntensity) 0.0 _light_track)))
        (:Finished
          (Actor|DestroyActor))))))

(fn ConstructionScript)

(fn MovetoPawn
  (params (self2 :type Actor%20Object%20Reference) (Alpha :type Float%20%28single-precision%29))
  (Transformation|SetActorLocation (Math|Vector|Lerp(Vector) (Variables|Default|GetStartLocation) (Transformation|GetActorLocation self2) Alpha) false false))

(fn GetStartValues
  (Variables|Default|SetStartLocation (Transformation|GetActorLocation))
  (Variables|Default|SetStartScale (Transformation|GetActorScale3D))
  (Variables|Default|SetStartIntensity (Variables|/Script/Engine.LightComponentBase|GetIntensity (Variables|Default|GetPointLight))))

(fn ScaleCrystal
  (params (Alpha :type Float%20%28single-precision%29))
  (Transformation|SetActorScale3D (Math|Vector|Lerp(Vector) (Variables|Default|GetStartScale) "0, 0, 0" Alpha)))