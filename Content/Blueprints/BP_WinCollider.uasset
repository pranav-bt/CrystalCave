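; BP_WinCollider is the level exit trigger that completes a level when the player overlaps it with every crystal collected.
; On overlap it counts remaining BP_Crystal actors and prints a reminder if any are left.
; Otherwise it finds the current level in the LevelNames array and opens the next one, or quits the game on the last level.
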(event Collision|EventActorBeginOverlap
  (params (OtherActor :type Actor%20Object%20Reference))
  (Utilities|IsPlayer OtherActor
    (:Player
      (if (CallFunction|CrystalsRemaining)
        (Development|PrintString "Collect All THe Gems First")
        (else
          (CallFunction|LevelComplete))))))

(fn ConstructionScript)

(fn CrystalsRemaining
  (bind _outactors (Actor|GetAllActorsOfClass "/Game/Blueprints/BP_Crystal.BP_Crystal_C"))
  (return (> (Utilities|Array|Length _outactors) 0)))

(fn LevelComplete
  (if (CallFunction|IsFinalLevel)
    (Game|QuitGame 0 "Quit" false)
    (else
      (CallFunction|LoadNextLevel))))

(fn GetCurrentLevelIndex
  (bind _returnvalue (Game|GetCurrentLevelName true))
  (return (Utilities|Array|FindItem (Variables|Default|GetLevelNames) (Utilities|String|StringToName _returnvalue))))

(fn IsFinalLevel
  (return (== (Utilities|Array|LastIndex (Variables|Default|GetLevelNames)) (CallFunction|GetCurrentLevelIndex))))

(fn LoadNextLevel
  (Game|OpenLevel(byName) (Utilities|Array|Get(acopy) (Variables|Default|GetLevelNames) (+ (CallFunction|GetCurrentLevelIndex) 1))))